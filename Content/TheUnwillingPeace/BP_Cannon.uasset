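; BP_Cannon is an interactable cannon the player aims and fires.
; Interact blends to the cannon camera, shows CannonUI and takes over input from the character; Inspect reverses this.
; MouseY pitches the barrel within limits (yaw is unwired), and firing spawns CannonBallBP with particles and camera shake.
; Each shot starts an overheat cooldown, with timelines driving the material's Heat parameter, while focus events toggle highlights and tooltip.
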(event `InputAction|Interact`
  (params (Key :type "Key Structure"))
  ;[1 1 1] Cannonball Shoot
  (:`Pressed`
    (if (`self.IsActive?`)
      (if (not (`self.Overheat`))
        (`self.ShootCannonBall`)
        ;[1 1 1] Camera Shake and shoot particles
        (`ActorComponent.Activate` (`self.Shoot Particle`) true)
        (`GameplayStatics.PlayWorldCameraShake` "/Game/TheUnwillingPeace/CameraCannonShake.CameraCannonShake_C" (`self.K2_GetActorLocation`) 0.0 6000.0)
        ;[1 1 1] Overheat Delay
        (set `self.Overheat` true)
        (bind (_direction _heatramp) (`Timeline|Timeline_0` :!via `PlayFromStart`)
          (:`Update`
            (`MeshComponent.SetScalarParameterValueOnMaterials` (`self.Cannon`) "Heat" _heatramp)
            (`|ExecutionSequence`
              (:`then_0`
                (bind (_direction_2 _heatramp_2) (`Timeline|Timeline_1` :!via `ReverseFromEnd`)
                  (:`Update`
                    (`MeshComponent.SetScalarParameterValueOnMaterials` (`self.Cannon`) "Heat" _heatramp_2))))
              (:`then_1`
                (`KismetSystemLibrary.Delay` 4.0)
                (set `self.Overheat` false)))))))))

(event `InputAxisKey|MouseY`
  (params (AxisValue :type "Float (single-precision)"))
  (bind _cannon (`self.Cannon`))
  (bind _pitch (.pitch (`SceneComponent.K2_GetComponentRotation` _cannon)))
  ;[1 1 1] Cannon Rotation
  (if (`self.IsActive?`)
    (if (or (and (> AxisValue 0.0) (< _pitch (`self.Max`))) (and (< AxisValue 0.0) (> _pitch (`self.Min`))))
      (`SceneComponent.K2_AddWorldRotation` _cannon (`KismetMathLibrary.MakeRotator` 0.0 AxisValue) false false))))

(event `InputAction|Inspect`
  (params (Key :type "Key Structure"))
  (bind _returnvalue (`GameplayStatics.GetPlayerController` 0))
  (bind _returnvalue_2 (`GameplayStatics.GetPlayerController` 0))
  ;[1 1 1] Camera Aim Out
  (:`Pressed`
    (if (`self.IsActive?`)
      (`PlayerController.SetViewTargetWithBlend` _returnvalue_2 (`Controller.K2_GetPawn` _returnvalue_2) 1.0 "VTBlend_EaseInOut" 2.0 false)
      (set `self.IsActive?` false)
      (`SceneComponent.SetVisibility` (`self.Fuse`) false false)
      (`SceneComponent.SetVisibility` (`self.Highlight`) false false)
      (`SceneComponent.SetVisibility` (`self.Highlight2`) false false)
      (`SceneComponent.SetVisibility` (`self.Tooltip`) false false)
      (`Widget.RemoveFromParent` (stale `self.ReceiveBeginPlay` _returnvalue))
      ;[1 1 1] Bug Fix For Input
      (`self.DisableInput` _returnvalue)
      (`self.EnableInput` (`GameplayStatics.GetPlayerCharacter` 0) _returnvalue))))

(event `self.ReceiveBeginPlay`
  ;[1 1 1] Widget
  (bind _returnvalue (`|CreateWidget` "/Game/TheUnwillingPeace/CannonUI.CannonUI_C" (`GameplayStatics.GetPlayerController` 0))))

(event `/Game/GamEngine/InteractionInterface.Interact`
  (bind _returnvalue (`GameplayStatics.GetPlayerController` 0))
  ;[1 1 1] Camera Aim In
  (if (not (`self.IsActive?`))
    (`PlayerController.SetViewTargetWithBlend` (`GameplayStatics.GetPlayerController` 0) (`self.Camera`) 1.0 "VTBlend_EaseInOut" 2.0 false)
    (set `self.IsActive?` true)
    (`SceneComponent.SetVisibility` (`self.Tooltip`) false false)
    (`SceneComponent.SetVisibility` (`self.Highlight2`) false false)
    (`SceneComponent.SetVisibility` (`self.Highlight`) false false)
    (`UserWidget.AddToViewport` (stale `self.ReceiveBeginPlay` _returnvalue) 0)
    (`SceneComponent.SetVisibility` (`self.Fuse`) true false)
    ;[1 1 1] Bug Fix For Input
    (`self.EnableInput` _returnvalue)
    (`self.DisableInput` (`GameplayStatics.GetPlayerCharacter` 0) _returnvalue)))

(event `InputAxisKey|MouseX`
  (params (AxisValue :type "Float (single-precision)"))
  (bind _yaw (.yaw (`SceneComponent.K2_GetComponentRotation` (`self.CannonCart`))))
  ;[1 1 1] Cannon Rotation
  (if (`self.IsActive?`)
    (if (or (and (> AxisValue 0.0) (< _yaw 13.0)) (and (< AxisValue 0.0) (> _yaw -23.0)))
      _)))

(event `/Game/GamEngine/InteractionInterface.OnFocus`
  ;[1 1 1] Highlight
  (if (not (`self.IsActive?`))
    (`SceneComponent.SetVisibility` (`self.Tooltip`) true false)
    (`SceneComponent.SetVisibility` (`self.Highlight`) true false)
    (`SceneComponent.SetVisibility` (`self.Highlight2`) true false)))

(event `/Game/GamEngine/InteractionInterface.OnBlur`
  ;[1 1 1] Highlight
  (`SceneComponent.SetVisibility` (`self.Tooltip`) false false)
  (`SceneComponent.SetVisibility` (`self.Highlight`) false false)
  (`SceneComponent.SetVisibility` (`self.Highlight2`) false false))

(fn `ShootCannonBall`
  (returns (`Cannonball Location` :type "Vector Structure"))
  (bind _returnvalue (`|SpawnActorFromClass` "/Game/TheUnwillingPeace/Effects/CannonBallBP.CannonBallBP_C" (`SceneComponent.K2_GetComponentToWorld` (`self.AimingDirection`)) "Undefined" "OverrideRootScale" null null))
  (return (`self.K2_GetActorLocation` _returnvalue)))

(fn `UserConstructionScript`)